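; Crafting machine that turns three ingredients into a coloured sweet, with keys 1–6 choosing the colour and starting the craft.
; It matches ingredient classes inside InputCollider against Recipies in any order by clearing matched slots on a working struct.
; A match spawns and initialises BP_Sweet, registers the recipe with BP_RecipeBook, then destroys the ingredients.
; The FoundSuccessfulRecipe reset sits in unconnected nodes, so the flag stays set after a match.
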(event Custom|OnActivate
  (params (ColourIndex :type Integer))
  (CallFunction|AssignColourfromIndex ColourIndex)
  (Development|PrintString "Start")
  (bind (_bisvalid _output) (CallFunction|ValidateInputs))
  (if _bisvalid
    (Variables|Default|SetCurrentIngredients _output)
    (for _array_element (Variables|Default|GetRecipies)
      (if (not (Variables|Default|GetbFoundSuccessfulRecipe))
        (bind _bsuccess (CallFunction|AssignRecipefromList (Variables|Default|GetCurrentIngredients) (Variables|Default|GetCreatedEffect)))
        (if _bsuccess
          (for _array_element_2 (Variables|Default|GetCurrentIngredients)
            (if (== _array_element_2 (.Ingredient1 (Utilities|Struct|BreakF_Recipe _array_element)))
              (Utilities|Struct|SetmembersinF_Recipe (Variables|Default|GetCreatedEffect) 0))
            (if (== _array_element_2 (.Ingredient2 (Utilities|Struct|BreakF_Recipe _array_element)))
              (Utilities|Struct|SetmembersinF_Recipe (Variables|Default|GetCreatedEffect) 0))
            (if (== _array_element_2 (.Ingredient3 (Utilities|Struct|BreakF_Recipe _array_element)))
              (Utilities|Struct|SetmembersinF_Recipe (Variables|Default|GetCreatedEffect) 0)))
          (if (not (Math|Boolean|ORBoolean (Utilities|IsValidClass (.ingredient1 (Variables|Default|GetCreatedEffect))) (Utilities|IsValidClass (.ingredient2 (Variables|Default|GetCreatedEffect))) (Utilities|IsValidClass (.ingredient3 (Variables|Default|GetCreatedEffect)))))
            (Variables|Default|SetCreatedEffect (Utilities|Struct|MakeF_Recipe (.Effect (Utilities|Struct|BreakF_Recipe _array_element)) (.Ingredient1 (Utilities|Struct|BreakF_Recipe _array_element)) (.Ingredient2 (Utilities|Struct|BreakF_Recipe _array_element)) (.Ingredient3 (Utilities|Struct|BreakF_Recipe _array_element)) (.Suspicion (Utilities|Struct|BreakF_Recipe _array_element))))
            (Variables|Default|SetbFoundSuccessfulRecipe true)
            (Development|PrintString (Utilities|String|Append "found " (Utilities|String|EnumtoString (.Effect (Utilities|Struct|BreakF_Recipe _array_element))) " as effect"))))))
    (CallFunction|FoundItem)
    (else
      (CallFunction|InvalidInputs))))

(event Custom|Invalid%20Inputs
  (Development|PrintString "ERROR: INVALID INPUTS" true true "(R=0.869792,G=0.559149,B=0.000000,A=1.000000)"))

(event Custom|FoundItem
  (bind _createdeffect (Variables|Default|GetCreatedEffect))
  ;[1 1 1] On Successful craft
  (if (Variables|Default|GetbFoundSuccessfulRecipe)
    (bind _returnvalue (Game|SpawnActorfromClass "/Game/MimiBuckler/BP_Sweet.BP_Sweet_C" (Math|Transform|MakeTransform (+ (Transformation|GetActorLocation) (Variables|Default|GetSpawnLocation)) "0, 0, 0" "1.000000,1.000000,1.000000") "Undefined" "MultiplyWithRoot" 0 0))
    (Default|Initialise _returnvalue false (.effect _createdeffect) (.suspicion _createdeffect) (Variables|Default|GetCurrentColour))
    (for (_array_element _array_index) (Collision|GetOverlappingActors (Variables|Default|GetInputCollider) "/Game/MimiBuckler/BP_Ingredient.BP_Ingredient_C" :!class /Script/Engine.PrimitiveComponent)
      (bind _asbp_ingredient (Utilities|Casting|CastToBP_Ingredient _array_element))
      (Utilities|Array|SetArrayElem (Variables|Default|GetDestroyArray) _array_index _asbp_ingredient true))
    ;[1 1 1] Sinful code, please forgive me
    (bind _returnvalue_2 (Actor|GetActorOfClass "/Game/MimiBuckler/BP_RecipeBook.BP_RecipeBook_C"))
    (Default|AddRecipe _returnvalue_2 (Variables|Default|GetDestroyArray) (Variables|Default|GetCreatedEffect))
    ;[1 1 1] Destroy ingredient actors, do last
    (for _array_element_2 (Variables|Default|GetDestroyArray)
      (Actor|DestroyActor _array_element_2))
    (else
      (Development|PrintString "No recipe found"))))

(event EventBeginPlay)

(event Collision|EventActorBeginOverlap
  (params (OtherActor :type Actor%20Object%20Reference)))

(event EventTick
  (params (DeltaSeconds :type Float%20%28single-precision%29)))

(event Input|KeyboardEvents|6
  (params (Key :type Key%20Structure :default "None"))
  (:Pressed
    (CallFunction|OnActivate 5)))

(event Input|KeyboardEvents|4
  (params (Key :type Key%20Structure :default "None"))
  (:Pressed
    (CallFunction|OnActivate 3)))

(event Input|KeyboardEvents|5
  (params (Key :type Key%20Structure :default "None"))
  (:Pressed
    (CallFunction|OnActivate 4)))

(event Input|KeyboardEvents|1
  (params (Key :type Key%20Structure :default "None"))
  (:Pressed
    (CallFunction|OnActivate)))

(event Input|KeyboardEvents|2
  (params (Key :type Key%20Structure :default "None"))
  (:Pressed
    (CallFunction|OnActivate 1)))

(event Input|KeyboardEvents|3
  (params (Key :type Key%20Structure :default "None"))
  (:Pressed
    (CallFunction|OnActivate 2)))

(fn ConstructionScript)

(fn ValidateInputs
  (bind _inputcollider (Variables|Default|GetInputCollider))
  (bind _overlappingactors (Collision|GetOverlappingActors _inputcollider "/Game/MimiBuckler/BP_Ingredient.BP_Ingredient_C" :!class /Script/Engine.PrimitiveComponent))
  (if (== (Utilities|Array|Length _overlappingactors) 3)
    (for _array_element _overlappingactors
      (bind _asbp_ingredient (Utilities|Casting|CastToBP_Ingredient _array_element))
      (Utilities|Array|Add (LocalVariables|GetvalidatedValues) (Utilities|GetClass _asbp_ingredient)))
    (return true (LocalVariables|GetvalidatedValues))
    (else
      (return false 0))))

(fn AssignRecipefromList
  (params (Inputs :type Array%20of%20Actor%20Class%20References) (Recipe :type F%20Recipe%20Structure%20%28by%20ref%29))
  (if (!= (Utilities|Array|Length Inputs) 3)
    (return false)
    (else
      (bind _asbp_ingredient (Utilities|Casting|CastToBP_IngredientClass (Utilities|Array|Get(acopy) Inputs))
        (:then
          (bind _asbp_ingredient_2 (Utilities|Casting|CastToBP_IngredientClass (Utilities|Array|Get(acopy) Inputs 1))
            (:then
              (bind _asbp_ingredient_3 (Utilities|Casting|CastToBP_IngredientClass (Utilities|Array|Get(acopy) Inputs 2))
                (:then
                  (|SetBy-RefVar Recipe (Utilities|Struct|MakeF_Recipe "NewEnumerator0" _asbp_ingredient_3 _asbp_ingredient_2 _asbp_ingredient 0.0))
                  (return true))
                (:CastFailed
                  _)))
            (:CastFailed
              _)))
        (:CastFailed
          _))
      (return false))))

(fn AssignColourfromIndex
  (params (Index :type Integer))
  (Variables|Default|SetCurrentColour (Utilities|Array|Get(acopy) (Variables|Default|GetColorList) Index)))