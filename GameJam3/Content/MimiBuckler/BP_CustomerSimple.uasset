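; Customer actor that gets random body and eye materials, judges a given sweet by colour and reacts to its effect.
; GiveRequest updates score and a save-object high score (never written to slot) on a match, then, right or wrong, leaves CustomerManager and runs the effect.
; Effects use Niagara, physics impulses and timelines, usually followed by a delayed queue shuffle and destroy.
; Some effects are stubs or unwired; P/O/I keys trigger three directly.
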(event Custom|GiveRequest
  (params (Sweet :type BP%20Sweet%20Object%20Reference))
  (bind _score (Variables|Default|Getscore))
  (bind _effect (Variables|/Game/MimiBuckler/BP_Sweet.BP_Sweet_C|GetEffect Sweet))
  (if (== (Variables|/Game/MimiBuckler/BP_Sweet.BP_Sweet_C|GetSweetColour Sweet) (Variables|Default|GetRequestedColour))
    ;[1 1 1] save game
    (Math|Integer|IncrementInt _score
      (:%20%20
        (if (>= _score (Variables|Default|GetHighScore))
          (bind _output_get (Variables|Default|SetHighScore (Variables|Default|Getscore)))
          (bind _returnvalue (SaveGame|DoesSaveGameExist "1"))
          (if _returnvalue
            (bind _returnvalue_2 (SaveGame|LoadGamefromSlot "1"))
            (bind _output_get_2 (Variables|Default|SetSaverSubclass _returnvalue_2))
            (bind _assavegame_hs (Utilities|Casting|CastTosavegame_hs _output_get_2))
            (Variables|/Game/Eddies_Stuff/savegame_hs.savegame_hs_C|Sethigh%20score _assavegame_hs _output_get)
            (else
              (bind _returnvalue_3 (SaveGame|CreateSaveGameObject "/Game/Eddies_Stuff/savegame_hs.savegame_hs_C"))
              (bind _output_get_3 (Variables|Default|SetSaverSubclass _returnvalue_3))
              (bind _assavegame_hs_2 (Utilities|Casting|CastTosavegame_hs _output_get_3))
              (Variables|/Game/Eddies_Stuff/savegame_hs.savegame_hs_C|Sethigh%20score _assavegame_hs_2 _output_get))))
        (Development|PrintString "Succeessful order")))
    (else
      (Development|PrintString "Unsucceessful order")))
  (Default|RemoveCustomer (Variables|Default|GetCustomerManager) self)
  (if (Utilities|Enum|Equal(Enum) _effect "NewEnumerator0")
    (CallFunction|EffectShit)
    (Utilities|FlowControl|Delay 5.0 :!label _label)
    (Default|Shuffle (Variables|Default|GetCustomerManager))
    (Actor|DestroyActor)
    (elif (Utilities|Enum|Equal(Enum) _effect "NewEnumerator1")
      (CallFunction|EffectHallucinate)
      (goto _label)
      (elif (Utilities|Enum|Equal(Enum) _effect "NewEnumerator2")
        (CallFunction|EffectLevitate 1.0)
        (goto _label)
        (elif (Utilities|Enum|Equal(Enum) _effect "NewEnumerator3")
          (Physics|SetSimulatePhysics (Variables|Default|GetSkeletalMesh) true)
          (Development|PrintString "Eddie's code here")
          (goto _label)
          (elif (Utilities|Enum|Equal(Enum) _effect "NewEnumerator4")
            (Development|PrintString "Eddie's code here")
            (goto _label)
            (elif (Utilities|Enum|Equal(Enum) _effect "NewEnumerator5")
              (CallFunction|EffectShrink)
              (goto _label)
              (elif (Utilities|Enum|Equal(Enum) _effect "NewEnumerator6")
                (CallFunction|EffectParalyse)
                (goto _label)))))))))

(event Custom|mince
  (bind _in_bone_name (Variables|Default|GetIn%20Bone%20Name))
  ;[1 1 1] expolde
  (for _index (range 0 (Utilities|Array|LastIndex _in_bone_name))
    (Class|SkeletalMeshComponent|BreakConstraint (Variables|Default|GetSkeletalMesh) "0, 0, 0" "0, 0, 0" (Utilities|Array|Get(acopy) _in_bone_name _index))
    (Utilities|FlowControl|Delay 2.0)
    (Actor|DestroyActor)))

(event Custom|Skinny%20Effect
  (bind _returnvalue (Transformation|GetActorTransform))
  ;[1 1 1] skinny
  (bind _newtrack_0 (Timeline|skinny PlayFromStart)
    (:Update
      (Transformation|SetActorTransform (Math|Transform|MakeTransform (.location _returnvalue) (.rotation _returnvalue) (Math|Vector|MakeVector (.x (.scale _returnvalue)) _newtrack_0 (.z (.scale _returnvalue))))))))

(event Custom|effect%20fat
  (bind _self self)
  (bind _returnvalue (Transformation|GetActorTransform _self))
  ;[1 1 1] Effect fat
  (bind (_direction _newtrack_0 _newtrack_1) (Timeline|fat PlayFromStart)
    (:Update
      (Transformation|SetActorTransform (Math|Transform|MakeTransform (.location _returnvalue) (.rotation _returnvalue) (Math|Vector|MakeVector _newtrack_1 _newtrack_0 (.z (.scale _returnvalue))))))))

(event Custom|EffectShrink
  ;[1 1 1] Shrink
  (bind _shrink (Timeline|Shrink Play)
    (:Update
      (Transformation|SetWorldScale3D (Variables|Default|GetSkeletalMesh) (Math|Conversions|ToVector(Float) (Math|Float|Lerp 2e+01 0.0 _shrink))))
    (:Finished
      (Actor|DestroyActor))))

(event Collision|EventActorBeginOverlap
  (params (OtherActor :type Actor%20Object%20Reference)))

(event EventTick
  (params (DeltaSeconds :type Float%20%28single-precision%29)))

(event EventBeginPlay
  (bind _skeletalmesh (Variables|Default|GetSkeletalMesh))
  ;[1 1 1] picks random meh then material mat values need to be updated tomorrow!!!!!!!!!!!!!!!!!!!!!!!!!!!!!!!!!!!
  (Rendering|Material|SetMaterial _skeletalmesh 1 (.OutItem (Utilities|Array|Random (Variables|Default|Getnewmateriahuman2lEYES_0))))
  (Rendering|Material|SetMaterial _skeletalmesh 0 (.OutItem (Utilities|Array|Random (Variables|Default|GetnewmaterialHuman2BODY_0)))))

(event Input|KeyboardEvents|I
  (params (Key :type Key%20Structure :default "None"))
  (:Pressed
    (CallFunction|EffectShrink)))

(event Input|KeyboardEvents|P
  (params (Key :type Key%20Structure :default "None"))
  (:Pressed
    (CallFunction|EffectParalyse)))

(event Input|KeyboardEvents|O
  (params (Key :type Key%20Structure :default "None"))
  (:Pressed
    (CallFunction|EffectLevitate 1.0)))

(fn ConstructionScript)

(fn EffectShit
  (Components|Activation|Activate (Variables|Default|GetNiagara) false))

(fn EffectHallucinate
  (Development|PrintString "Move UVs"))

(fn EffectLevitate
  (params (Speed :type Float%20%28double-precision%29))
  (Physics|SetSimulatePhysics (Variables|Default|GetSkeletalMesh) true)
  (Physics|AddImpulse (Variables|Default|GetSkeletalMesh) (Math|Vector|MakeVector 0.0 0.0 (* (Math|Float|Clamp(Float) Speed 0.1 1e+02) 1e+04)) "None" false))

(fn EffectParalyse
  (bind _box (Variables|Default|GetBox))
  (Transformation|AttachComponentToComponent (Variables|Default|GetSkeletalMesh) (Variables|Default|GetBox) "None" "SnapToTarget" "SnapToTarget" "KeepRelative" true)
  (Physics|SetSimulatePhysics _box true)
  (Physics|SetEnableGravity _box true)
  (Physics|AddImpulseatLocation (Variables|Default|GetBox) (Math|Vector|MakeVector 0.0 0.0 1e+04) (Math|Vector|MakeVector 1e+01 1e+01 -2e+02) "None"))

(fn EffectSelfDetonate
  (Components|Animation|PlayAnimation (Variables|Default|GetSkeletalMesh) 0 false)
  (Components|Activation|Activate (Variables|Default|Getfire) false))

(fn Detonate
  (Components|Activation|Activate (Variables|Default|Getfire) false)
  (Actor|DestroyActor))