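; Recipe book actor that displays crafted recipes as lines of 3D text.
; On BeginPlay it caches the TextRender children of Title as a pool of lines.
; AddRecipe fills and reveals the next line with three ingredient names and the NewRecipe effect.
; A timeline then animates that line's height through HeightLerp, advancing the recipe count when finished.
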(event Custom|Add%20Recipe
  (params (Ingredients :type Array%20of%20BP%20Ingredient%20Object%20References) (New%20Recipe :type F%20Recipe%20Structure))
  (bind _currentrecipecount (Variables|Default|GetCurrentRecipeCount))
  (bind _textcomponents (Variables|Default|GetTextComponents))
  (bind _output (Utilities|Array|Get(acopy) _textcomponents _currentrecipecount))
  ;[0 0.05518 1] Turns craft into text - Bless this mess
  (Rendering|Components|TextRender|SetText _output (Utilities|Text|ToText(String) (Utilities|String|Append (Variables|/Game/MimiBuckler/BP_Ingredient.BP_Ingredient_C|GetDisplayName (Utilities|Array|Get(acopy) Ingredients)) " + " (Variables|/Game/MimiBuckler/BP_Ingredient.BP_Ingredient_C|GetDisplayName (Utilities|Array|Get(acopy) Ingredients 1)) " + " (Variables|/Game/MimiBuckler/BP_Ingredient.BP_Ingredient_C|GetDisplayName (Utilities|Array|Get(acopy) Ingredients 2)) " = " (Utilities|String|EnumtoString (.effect New%20Recipe)))))
  (Development|SetHiddeninGame _output false false)
  (bind _t (Timeline|Lerp%20Timeline Play)
    (:Update
      (Transformation|SetRelativeLocation _output (Math|Vector|MakeVector 0.0 0.0 (|HeightLerp _t)) false false))
    (:Finished
      (Math|Integer|IncrementInt (Variables|Default|GetCurrentRecipeCount)))))

(event Collision|EventActorBeginOverlap
  (params (OtherActor :type Actor%20Object%20Reference)))

(event EventTick
  (params (DeltaSeconds :type Float%20%28single-precision%29)))

(event EventBeginPlay
  (for _array_element (Components|GetChildrenComponents (Variables|Default|GetTitle) false)
    (bind _astext_render_component (Utilities|Casting|CastToTextRenderComponent _array_element))
    (Utilities|Array|Add (Variables|Default|GetTextComponents) _astext_render_component)))

(fn ConstructionScript)