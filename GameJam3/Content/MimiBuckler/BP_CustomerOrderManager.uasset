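; BP_CustomerOrderManager is an interactable counter that runs the customer order loop for selling sweets.
; It spawns one customer at a time with a random requested colour from a master list and shows that colour on the HUD.
; Interacting while holding a sweet passes its colour to the current customer and takes it from the player.
; Removing a customer destroys it, updates HUD suspicion from the last sweet, then spawns the next.
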(event Custom|NewCustomer
  ;[1 1 1] Spawn new customer
  (bind _returnvalue (Game|SpawnActorfromClass "/Game/MimiBuckler/BP_CustomerSimple.BP_CustomerSimple_C" (Math|Transform|MakeTransform (Variables|Default|GetCustomerSpawnPositionOrigin) "0, 0, 0" "1.000000,1.000000,1.000000") "Undefined" "MultiplyWithRoot" 0 0))
  (Utilities|Array|Add (Variables|Default|GetCustomers) _returnvalue)
  (bind _output_get (Variables|/Game/MimiBuckler/BP_CustomerSimple.BP_CustomerSimple_C|SetRequestedColour _returnvalue (.OutItem (Utilities|Array|Random (Variables|Default|GetMasterColorList)))))
  (Variables|/Game/MimiBuckler/BP_CustomerSimple.BP_CustomerSimple_C|SetCustomerManager _returnvalue self)
  (Variables|/Game/MimiBuckler/WBP_HUD.WBP_HUD_C|SetCurrentSweetColour (Variables|Default|GetHUD) _output_get))

(event Custom|SellSweet
  (params (Sweet :type BP%20Sweet%20Object%20Reference))
  ;[1 1 1] Sell the sweet
  (bind _output_get (Variables|Default|SetCurrentSweet Sweet))
  (Default|GiveRequest (Utilities|Array|Get(acopy) (Variables|Default|GetCustomers)) (Variables|/Game/MimiBuckler/BP_Sweet.BP_Sweet_C|GetSweetColour _output_get)))

(event Custom|RemoveCustomer
  (params (CustomerToRemove :type BP%20Customer%20Simple%20Object%20Reference))
  ;[1 1 1] Remove customer
  (Utilities|Array|RemoveItem (Variables|Default|GetCustomers) CustomerToRemove)
  (Actor|DestroyActor CustomerToRemove)
  (Utilities|FlowControl|Delay 1.0)
  (Default|UpdateSuspicion (Variables|Default|GetHUD) (Variables|/Game/MimiBuckler/BP_Sweet.BP_Sweet_C|GetSuspicion (Variables|Default|GetCurrentSweet)))
  (CallFunction|NewCustomer))

(event EventBeginPlay
  (Utilities|FlowControl|Delay 0.1)
  (bind _foundwidgets (Widget|GetAllWidgetsOfClass "/Game/MimiBuckler/WBP_HUD.WBP_HUD_C" true))
  (Variables|Default|SetHUD (Utilities|Array|Get(acopy) _foundwidgets))
  (CallFunction|NewCustomer))

(fn ConstructionScript)

(fn OnInteract
  (params (HitComponent :type Primitive%20Component%20Object%20Reference))
  (bind _asbp_first_person_character (Utilities|Casting|CastToBP_FirstPersonCharacter (Game|GetPlayerCharacter 0)))
  (bind _asbp_sweet (Utilities|Casting|CastToBP_Sweet (Variables|/Game/FirstPerson/Blueprints/BP_FirstPersonCharacter.BP_FirstPersonCharacter_C|GetCurrentPickup _asbp_first_person_character)))
  (CallFunction|SellSweet _asbp_sweet)
  (Default|ForceRemoveItem _asbp_first_person_character (+ (Variables|Default|GetSweetPosition) (Transformation|GetActorLocation)))
  (return self false))