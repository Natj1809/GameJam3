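; BP_Counter is a service counter that tracks which spots in its customer queue are occupied.
; The construction script caches order, fulfilled-order and queue placement positions and gathers customer spawners; Queue1–Q9 are set only inside the spawner loop.
; A looping timer runs QueueSystem, which checks ten boxes in order for Bpi_queue customers and flags them full.
; The nested checks stop at the first empty box, and nothing here clears the flags.
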(event Custom|refresh
  (CallFunction|QueueSystem))

(event EventBeginPlay
  (Utilities|Time|SetTimerbyEvent (delegate Custom|refresh) 0.1 true))

(fn ConstructionScript
  (Variables|Q|Setcustomer%20location (Transformation|GetWorldTransform (Variables|Default|Getcustomer%20placement)))
  (Variables|Default|SetOrder%20Location (Transformation|GetWorldLocation (Variables|Default|Getorder)))
  (Variables|Default|Setfufilled%20location (Transformation|GetWorldLocation (Variables|Default|Getfufilled%20order)))
  (bind _outactors (Actor|GetAllActorsOfClass "/Game/Eddies_Stuff/BP_CustomerSpawn.BP_CustomerSpawn_C"))
  (for _array_element _outactors
    (Utilities|Array|Add (Variables|Default|Getcustomer%20spawn) _array_element)
    (Variables|q|Setqueue1 (Transformation|GetWorldTransform (Variables|Default|Getcustomer%20placement1)))
    (Variables|q|Setqueue%202 (Transformation|GetWorldTransform (Variables|Default|Getcustomer%20placement2)))
    (Variables|Q|Setq%203 (Transformation|GetWorldTransform (Variables|Default|Getcustomer%20placement3)))
    (Variables|Q|Setq%204 (Transformation|GetWorldTransform (Variables|Default|Getcustomer%20placement4)))
    (Variables|Q|Setq%205 (Transformation|GetWorldTransform (Variables|Default|Getcustomer%20placement5)))
    (Variables|Q|Setq%206 (Transformation|GetWorldTransform (Variables|Default|Getcustomer%20placement6)))
    (Variables|Q|Setq%207 (Transformation|GetWorldTransform (Variables|Default|Getcustomer%20placement7)))
    (Variables|Q|Setq%208 (Transformation|GetWorldTransform (Variables|Default|Getcustomer%20placement8)))
    (Variables|Q|Setq%209 (Transformation|GetWorldTransform (Variables|Default|Getcustomer%20placement9)))))

(fn QueueSystem
  (if (Utilities|DoesObjectImplementInterface (Utilities|Array|Get(acopy) (Collision|GetOverlappingActors (Variables|Default|GetBox1) "/Game/Eddies_Stuff/bp_customer.bp_customer_C" :!class /Script/Engine.PrimitiveComponent)) "/Game/Eddies_Stuff/bpi_queue.bpi_queue_C")
    (Variables|qfull|Setq1full? true)
    (if (Utilities|DoesObjectImplementInterface (Utilities|Array|Get(acopy) (Collision|GetOverlappingActors (Variables|Default|GetBox2) "/Game/Eddies_Stuff/bp_customer.bp_customer_C" :!class /Script/Engine.PrimitiveComponent)) "/Game/Eddies_Stuff/bpi_queue.bpi_queue_C")
      (Variables|Qfull|Setq2full? true)
      (if (Utilities|DoesObjectImplementInterface (Utilities|Array|Get(acopy) (Collision|GetOverlappingActors (Variables|Default|GetBox3) "/Game/Eddies_Stuff/bp_customer.bp_customer_C" :!class /Script/Engine.PrimitiveComponent)) "/Game/Eddies_Stuff/bpi_queue.bpi_queue_C")
        (Variables|Qfull|Setqfull3 true)
        (if (Utilities|DoesObjectImplementInterface (Utilities|Array|Get(acopy) (Collision|GetOverlappingActors (Variables|Default|GetBox4) "/Game/Eddies_Stuff/bp_customer.bp_customer_C" :!class /Script/Engine.PrimitiveComponent)) "/Game/Eddies_Stuff/bpi_queue.bpi_queue_C")
          (Variables|Qfull|Setqfull4 true)
          (if (Utilities|DoesObjectImplementInterface (Utilities|Array|Get(acopy) (Collision|GetOverlappingActors (Variables|Default|GetBox5) "/Game/Eddies_Stuff/bp_customer.bp_customer_C" :!class /Script/Engine.PrimitiveComponent)) "/Game/Eddies_Stuff/bpi_queue.bpi_queue_C")
            (Variables|Qfull|Setqfull5 true)
            (if (Utilities|DoesObjectImplementInterface (Utilities|Array|Get(acopy) (Collision|GetOverlappingActors (Variables|Default|GetBox6) "/Game/Eddies_Stuff/bp_customer.bp_customer_C" :!class /Script/Engine.PrimitiveComponent)) "/Game/Eddies_Stuff/bpi_queue.bpi_queue_C")
              (Variables|Qfull|Setqfull6 true)
              (if (Utilities|DoesObjectImplementInterface (Utilities|Array|Get(acopy) (Collision|GetOverlappingActors (Variables|Default|GetBox7) "/Game/Eddies_Stuff/bp_customer.bp_customer_C" :!class /Script/Engine.PrimitiveComponent)) "/Game/Eddies_Stuff/bpi_queue.bpi_queue_C")
                (Variables|Qfull|Setqfull7 true)
                (if (Utilities|DoesObjectImplementInterface (Utilities|Array|Get(acopy) (Collision|GetOverlappingActors (Variables|Default|GetBox8) "/Game/Eddies_Stuff/bp_customer.bp_customer_C" :!class /Script/Engine.PrimitiveComponent)) "/Game/Eddies_Stuff/bpi_queue.bpi_queue_C")
                  (Variables|Qfull|Setqfull8 true)
                  (if (Utilities|DoesObjectImplementInterface (Utilities|Array|Get(acopy) (Collision|GetOverlappingActors (Variables|Default|GetBox9) "/Game/Eddies_Stuff/bp_customer.bp_customer_C" :!class /Script/Engine.PrimitiveComponent)) "/Game/Eddies_Stuff/bpi_queue.bpi_queue_C")
                    (Variables|Qfull|Setqfull9 true)
                    (if (Utilities|DoesObjectImplementInterface (Utilities|Array|Get(acopy) (Collision|GetOverlappingActors (Variables|Default|GetBox10) "/Game/Eddies_Stuff/bp_customer.bp_customer_C" :!class /Script/Engine.PrimitiveComponent)) "/Game/Eddies_Stuff/bpi_queue.bpi_queue_C")
                      (Variables|Qfull|Setqfull10 true))))))))))))