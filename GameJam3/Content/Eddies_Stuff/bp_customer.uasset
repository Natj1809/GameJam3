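; Customer pawn meant to queue at a counter and place an order, though that logic is disconnected and BeginPlay does nothing.
; The unwired chain walks to the first free counter slot via nested queue-flag checks, spawning an order and looping a "leave" timer at the front.
; Leave checks the player's OrderPlaced, moves the first customer and frees the front slot.
; Nested construction-script loops cache counters, players and orders; Despawn destroys the actor.
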(event Custom|leave
  (if (Variables|/Game/FirstPerson/Blueprints/BP_FirstPersonCharacter.BP_FirstPersonCharacter_C|GetOrder%20Placed? (Utilities|Array|Get(acopy) (Variables|Default|Getcharacter)))
    (AI|AIMoveTo (Utilities|Array|Get(acopy) (Variables|Default|Getcustomer)) "0, 0, 0" 0 5.0 false
      (:then
        ;[1 1 1] Moves the customer to the counter then sets their order down
        (Variables|/Game/Eddies_Stuff/BP_Counter.BP_Counter_C|Setq1full? (Utilities|Array|Get(acopy) (Variables|Default|Getcounter)) false)))))

(event Custom|Despawn
  (Actor|DestroyActor))

(event EventBeginPlay
  ;[1 1 1] Moves the customer to the counter then sets their order down
)

(fn ConstructionScript
  (bind _outactors (Actor|GetAllActorsOfClass "/Game/Eddies_Stuff/BP_Counter.BP_Counter_C"))
  (for _array_element _outactors
    (Utilities|Array|Add (Variables|Default|Getcounter) _array_element)
    (bind _outactors_2 (Actor|GetAllActorsOfClass "/Game/FirstPerson/Blueprints/BP_FirstPersonCharacter.BP_FirstPersonCharacter_C"))
    (for _array_element_2 _outactors_2
      (Utilities|Array|Add (Variables|Default|Getcharacter) _array_element_2)
      (bind _outactors_3 (Actor|GetAllActorsOfClass "/Game/Eddies_Stuff/BP_Order.BP_Order_C"))
      (for _array_element_3 _outactors_3
        (Utilities|Array|Add (Variables|Default|Getorders) _array_element_3)))))