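; BP_CustomerSpawn is a spawner actor that brings Bp_customer actors into the game at its arrow's transform.
; BeginPlay starts a looping timer, its interval randomised once between min and max spawn times, that calls SpawnCustomers.
; That event appends each new customer to Customers, or pauses the timer at ten or more; only its spawn branch unpauses it.
; The construction script caches the arrow transform and seeds Customers with existing customers.
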(event Custom|Spawn%20Customers
  ;[1 1 1] if more than 10 customers are in the queue it pauses the timer stopping more customers from entering
  (if (>= (Utilities|Array|Length (Variables|Default|Getcustomers)) 10)
    (Utilities|Time|PauseTimerbyHandle (stale EventBeginPlay _returnvalue))
    (else
      ;[1 1 1] starts the customers entering and adds them to the array
      (Utilities|Time|UnpauseTimerbyHandle (stale EventBeginPlay _returnvalue))
      (bind _returnvalue (Game|SpawnActorfromClass "/Game/Eddies_Stuff/bp_customer.bp_customer_C" (Variables|Default|Getarrow%20location) "AdjustIfPossibleButAlwaysSpawn" "MultiplyWithRoot" 0 0))
      (Utilities|Array|Add (Variables|Default|Getcustomers) _returnvalue))))

(event EventBeginPlay
  ;[1 1 1] sets timer going to spawn customers
  (bind _returnvalue (Utilities|Time|SetTimerbyEvent (delegate Custom|Spawn%20Customers) (Math|Random|RandomFloatinRange (Variables|Default|GetMin%20spawn%20time) (Variables|Default|GetMax%20spawn%20time)) true)))

(event Collision|EventActorBeginOverlap
  (params (OtherActor :type Actor%20Object%20Reference)))

(event EventTick
  (params (DeltaSeconds :type Float%20%28single-precision%29)))

(fn ConstructionScript
  (Variables|Default|Setarrow%20location (Transformation|GetWorldTransform (Variables|Default|GetArrow)))
  (bind _outactors (Actor|GetAllActorsOfClass "/Game/Eddies_Stuff/bp_customer.bp_customer_C"))
  (for _array_element _outactors
    (Utilities|Array|Add (Variables|Default|Getcustomers) _array_element)))