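; BP_Order is an order display actor whose mesh shows the colour currently requested by the counter.
; The construction script caches the first BP_Conter found in the level as Counter.
; On BeginPlay, SetColour runs once, matching the counter's RequestedColour exactly against six fixed colours to pick the mesh material.
; SetColour ignores its colour input, and an unmatched colour leaves the material unchanged.
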(event EventBeginPlay
  (CallFunction|SetColour))

(fn ConstructionScript
  (bind _returnvalue (Actor|GetActorOfClass "/Game/Eddies_Stuff/newstuff/BP_Conter.BP_Conter_C"))
  (Variables|Default|Setcounter _returnvalue))

(fn SetColour
  (params (InputPin :type Linear%20Color%20Structure))
  (bind _counter (Variables|Default|Getcounter))
  (bind _requested_colour (Variables|/Game/Eddies_Stuff/newstuff/BP_Conter.BP_Conter_C|Getrequested%20colour _counter))
  (if (== _requested_colour "(R=0.474796,G=0.004898,B=0.608333,A=1.000000)")
    (Rendering|Material|SetMaterial (Variables|Default|GetStaticMesh) 0 "/Game/Eddies_Stuff/orderMeshAndTextures/purple/M_orderPurple.M_orderPurple")
    (elif (== _requested_colour "(R=0.000000,G=0.085981,B=1.000000,A=1.000000)")
      (Rendering|Material|SetMaterial (Variables|Default|GetStaticMesh) 0 "/Game/Eddies_Stuff/orderMeshAndTextures/blue/M_orderBlue.M_orderBlue")
      (elif (== _requested_colour "(R=1.000000,G=0.000000,B=0.000000,A=1.000000)")
        (Rendering|Material|SetMaterial (Variables|Default|GetStaticMesh) 0 "/Game/Eddies_Stuff/orderMeshAndTextures/red/M_OrderRed.M_OrderRed")
        (elif (== _requested_colour "(R=0.000000,G=0.671875,B=0.071850,A=1.000000)")
          (Rendering|Material|SetMaterial (Variables|Default|GetStaticMesh) 0 "/Game/Eddies_Stuff/orderMeshAndTextures/green/M_OrderGreen.M_OrderGreen")
          (elif (== _requested_colour "(R=1.000000,G=0.889721,B=0.000000,A=1.000000)")
            (Rendering|Material|SetMaterial (Variables|Default|GetStaticMesh) 0 "/Game/Eddies_Stuff/orderMeshAndTextures/yellow/M_orderYellow.M_orderYellow")
            (elif (== _requested_colour "(R=0.021000,G=0.021000,B=0.021000,A=1.000000)")
              (Rendering|Material|SetMaterial (Variables|Default|GetStaticMesh) 0 "/Game/Eddies_Stuff/orderMeshAndTextures/black/M_OrderBlack.M_OrderBlack"))))))))