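; BP_Lift is an interactable lift that moves when the player interacts with it.
; OnInteract calls Move, where a FlipFlop alternates between two timelines that drive the Lift component's relative Z.
; Player input is disabled during each ride and restored when the timeline finishes.
; The construction script caches an arrow's location as PlaceMeHere, used only by an unconnected SimpleMoveToLocation branch.
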(event Custom|move
  (bind _returnvalue (Game|GetPlayerController 0))
  (Utilities|FlowControl|FlipFlop
    (:A
      (bind _asbp_first_person_character (Utilities|Casting|CastToBP_FirstPersonCharacter (Game|GetPlayerCharacter 0)))
      (bind _output_get (Variables|Default|SetAs%20BP%20First%20Person%20Character _asbp_first_person_character))
      (Input|DisableInput _output_get _returnvalue)
      (bind _newtrack_0 (Timeline|Timeline PlayFromStart)
        (:Update
          (Transformation|SetRelativeLocation (Variables|Default|Getlift) (Math|Vector|MakeVector 0.0 0.0 _newtrack_0) false false))
        (:Finished
          (Input|EnableInput _output_get _returnvalue))))
    (:B
      (Input|DisableInput (Variables|Default|GetAs%20BP%20First%20Person%20Character) _returnvalue)
      (bind _newtrack_0_2 (Timeline|Timeline_0 PlayFromStart)
        (:Update
          (Transformation|SetRelativeLocation (Variables|Default|Getlift) (Math|Vector|MakeVector 0.0 0.0 _newtrack_0_2) false false))
        (:Finished
          (Input|EnableInput (Variables|Default|GetAs%20BP%20First%20Person%20Character) _returnvalue))))))

(fn ConstructionScript
  (Variables|Default|Setplace%20me%20here (Transformation|GetWorldLocation (Variables|Default|GetArrow))))

(fn OnInteract
  (params (HitComponent :type Primitive%20Component%20Object%20Reference))
  (CallFunction|Move)
  (return self false))