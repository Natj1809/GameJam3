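; A queue Blueprint that defines nine world positions through arrow components, likely spots for actors waiting in line.
; The Construction Script caches each arrow's world location in its own variable.
; BeginPlay adds those variables to the Positions array in a fixed order that starts with Position5 rather than Position1.
; The Blueprint only builds this list and contains no logic for assigning or moving occupants.
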(event EventBeginPlay
  (Utilities|Array|Add (Variables|Default|Getpositions) (Variables|Default|Getposition%205))
  (Utilities|Array|Add (Variables|Default|Getpositions) (Variables|Default|Getposition%201))
  (Utilities|Array|Add (Variables|Default|Getpositions) (Variables|Default|Getpositio%202))
  (Utilities|Array|Add (Variables|Default|Getpositions) (Variables|Default|Getposition%203))
  (Utilities|Array|Add (Variables|Default|Getpositions) (Variables|Default|Getposition%204))
  (Utilities|Array|Add (Variables|Default|Getpositions) (Variables|Default|Getpos%206))
  (Utilities|Array|Add (Variables|Default|Getpositions) (Variables|Default|Getpos%207))
  (Utilities|Array|Add (Variables|Default|Getpositions) (Variables|Default|Getpos%208))
  (Utilities|Array|Add (Variables|Default|Getpositions) (Variables|Default|Getpos%209)))

(event EventTick
  (params (DeltaSeconds :type Float%20%28single-precision%29)))

(fn ConstructionScript
  (Variables|Default|Setposition%205 (Transformation|GetWorldLocation (Variables|Default|GetArrow8)))
  (Variables|Default|Setposition%201 (Transformation|GetWorldLocation (Variables|Default|GetArrow2)))
  (Variables|Default|Setpositio%202 (Transformation|GetWorldLocation (Variables|Default|GetArrow1)))
  (Variables|Default|Setposition%203 (Transformation|GetWorldLocation (Variables|Default|GetArrow3)))
  (Variables|Default|Setposition%204 (Transformation|GetWorldLocation (Variables|Default|GetArrow)))
  (Variables|Default|Setpos%206 (Transformation|GetWorldLocation (Variables|Default|GetArrow7)))
  (Variables|Default|Setpos%207 (Transformation|GetWorldLocation (Variables|Default|GetArrow4)))
  (Variables|Default|Setpos%208 (Transformation|GetWorldLocation (Variables|Default|GetArrow5)))
  (Variables|Default|Setpos%209 (Transformation|GetWorldLocation (Variables|Default|GetArrow6))))