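; Shop counter actor that runs a queue of up to four Cop customers, who place colour orders.
; A looping timer spawns a customer while there is room, then re-issues AI moves sending each to its queue slot, cached from components at BeginPlay.
; Each front-customer move re-rolls the requested colour and, on success, spawns a BP_Order.
; The door-rotation timeline and customer/order cleanup logic are unwired, so the queue never empties here.
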(event Custom|spawn
  (bind _customers_in_level (CallFunction|AcchualSpawn))
  (for (_array_element _array_index) _customers_in_level
    (if (== _array_index 0)
      (AI|AIMoveTo _array_element (Utilities|Array|Get(acopy) (Variables|Locations|Getqueue%20locations)) 0 5.0 false
        (:then
          (Variables|Default|Setrequested%20colour (.OutItem (Utilities|Array|Random (Variables|Default|Getmaster%20colour%20list)))))
        (:OnSuccess
          (bind _returnvalue (Game|SpawnActorfromClass "/Game/Eddies_Stuff/BP_Order.BP_Order_C" (Math|Transform|MakeTransform (Variables|Locations|Getorder%20loc) "0, 0, 0" "1.000000,1.000000,1.000000") "AdjustIfPossibleButAlwaysSpawn" "MultiplyWithRoot" 0 0))
          (Utilities|Array|Add (Variables|Default|Getdead%20orders) _returnvalue)))
      (elif (== _array_index 1)
        (AI|AIMoveTo _array_element (Variables|Locations|Getq2%20loc) 0 5.0 false)
        (elif (== _array_index 2)
          (AI|AIMoveTo _array_element (Variables|Locations|Getq3%20loc) 0 5.0 false)
          (elif (== _array_index 3)
            (AI|AIMoveTo _array_element (Variables|Locations|Getq4%20loc) 0 5.0 false)))))))

(event EventBeginPlay
  (Utilities|FlowControl|Delay 0.2)
  (bind _foundwidgets (Widget|GetAllWidgetsOfClass "/Game/MimiBuckler/WBP_HUD.WBP_HUD_C" true))
  (Variables|Default|SetHUD (Utilities|Array|Get(acopy) _foundwidgets))
  (CallFunction|AddLocations)
  (Utilities|Time|SetTimerbyFunctionName 0 "spawn" 3.0 true))

(fn ConstructionScript)

(fn AddLocations
  (bind _queue_locations (Variables|Locations|Getqueue%20locations))
  (Variables|locations|Setq1%20loc (Transformation|GetWorldLocation (Variables|Default|Getq1)))
  (Variables|Locations|Setq2%20loc (Transformation|GetWorldLocation (Variables|Default|Getq2)))
  (Variables|Locations|Setq3%20loc (Transformation|GetWorldLocation (Variables|Default|Getq3)))
  (Variables|Locations|Setq4%20loc (Transformation|GetWorldLocation (Variables|Default|Getq4)))
  (Variables|Locations|Setwonka%20loc (Transformation|GetWorldLocation (Variables|Default|Getwonka)))
  (Variables|Locations|Setorder%20loc (Transformation|GetWorldLocation (Variables|Default|Getorder%20request)))
  (Utilities|Array|Add _queue_locations (Variables|locations|Getq1%20loc))
  (Utilities|Array|Add _queue_locations (Variables|Locations|Getq2%20loc))
  (Utilities|Array|Add _queue_locations (Variables|Locations|Getq3%20loc))
  (Utilities|Array|Add _queue_locations (Variables|Locations|Getq4%20loc)))

(fn AcchualSpawn
  (bind _customers_in_level (Variables|Default|Getcustomers%20in%20level))
  (if (>= (Utilities|Array|Length (Variables|Default|Getcustomers%20in%20level)) 4)
    _
    (else
      (bind _returnvalue (Game|SpawnActorfromClass "/Game/Eddies_Stuff/newstuff/cop.cop_C" (Transformation|GetWorldTransform (Variables|Default|Getcustomer%20spawn)) "AdjustIfPossibleButAlwaysSpawn" "MultiplyWithRoot" 0 0))
      (Utilities|Array|Add _customers_in_level _returnvalue)
      (Utilities|Array|Add (Variables|Default|GetTo%20Kill) _returnvalue)))
  (return _customers_in_level))